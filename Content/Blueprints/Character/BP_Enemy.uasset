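; Enemy character that shoots at the player with an equipped weapon and drops loot on death.
; BeginPlay hides weapon bones, spawns EquipedWeapon at zero scale, and unhides the mesh bone matching its name.
; Fire shoots from that named socket toward player 0.
; At zero life, BeingHit plays a death montage, then drops the weapon pickup with its magazine plus type-matched ammo (Rocket gives pistol ammo) and destroys the actor.
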(event Custom|DropStuff
  (bind _returnvalue (Transformation|GetActorLocation))
  ;[1 1 1] Drop Stuff
  (if (Utilities|IsValid (Variables|Default|GetCurrentWeapon))
    (bind _returnvalue_2 (Game|SpawnActorfromClass (Variables|/Game/Blueprints/Props/Weapons/BP_WeaponMaster.BP_WeaponMaster_C|GetPickupClass (Variables|Default|GetCurrentWeapon)) (Math|Transform|MakeTransform (Math|Vector|MakeVector (.x _returnvalue) (.y _returnvalue) (+ (.z _returnvalue) 5e+01)) "0, 0, 0" "1.000000,1.000000,1.000000") "AlwaysSpawn" "MultiplyWithRoot" 0 0))
    (Variables|/Game/Blueprints/Props/Pickups/BP_WeaponPickup.BP_WeaponPickup_C|SetCurrentMagazine _returnvalue_2 (Variables|/Game/Blueprints/Props/Weapons/BP_WeaponMaster.BP_WeaponMaster_C|GetCurrentMagazine (Variables|Default|GetCurrentWeapon)))
    (CallFunction|DropAmmos)))

(event Custom|Fire
  ;[1 1 1] Fire
  (if (Variables|Default|GetIsAlive)
    (Default|Shoot (Variables|Default|GetCurrentWeapon) (Math|Rotator|FindLookatRotation (Transformation|GetActorLocation) (Transformation|GetActorLocation (Game|GetPlayerCharacter 0))) (Transformation|GetSocketLocation (Variables|Character|GetMesh) (Variables|/Game/Blueprints/Props/Weapons/BP_WeaponMaster.BP_WeaponMaster_C|GetName (Variables|Default|GetCurrentWeapon))))))

(event Custom|DropAmmos
  ;[0.05521 0.05521 0.05521] Drop Ammos
  (switch Utilities|FlowControl|Switch|SwitchonE_AmmoType (Variables|/Game/Blueprints/Props/Weapons/BP_WeaponMaster.BP_WeaponMaster_C|GetAmmoType (Variables|Default|GetCurrentWeapon))
    (:NewEnumerator0
      (CallFunction|SpawnAmmos "/Game/Blueprints/Props/Pickups/Ammo/BP_AmmoRiflePickup.BP_AmmoRiflePickup_C"))
    (:NewEnumerator1
      (CallFunction|SpawnAmmos "/Game/Blueprints/Props/Pickups/Ammo/BP_AmmoSMGPickup.BP_AmmoSMGPickup_C"))
    (:NewEnumerator2
      (CallFunction|SpawnAmmos "/Game/Blueprints/Props/Pickups/Ammo/BP_AmmoPistolPickup.BP_AmmoPistolPickup_C"))
    (:NewEnumerator3
      (CallFunction|SpawnAmmos "/Game/Blueprints/Props/Pickups/Ammo/BP_AmmoSniperPickup.BP_AmmoSniperPickup_C"))
    (:NewEnumerator4
      (CallFunction|SpawnAmmos "/Game/Blueprints/Props/Pickups/Ammo/BP_AmmoShotgunPickup.BP_AmmoShotgunPickup_C"))
    (:NewEnumerator5
      (CallFunction|SpawnAmmos "/Game/Blueprints/Props/Pickups/Ammo/BP_AmmoPistolPickup.BP_AmmoPistolPickup_C"))))

(event Custom|SpawnAmmos
  (params (AmmoClass :type BP%20Ammo%20Pickup%20Class%20Reference))
  (bind _returnvalue (Transformation|GetActorLocation))
  ;[0.03854 0.03854 0.03854] Spawn Ammos
  (Game|SpawnActorfromClass AmmoClass (Math|Transform|MakeTransform (Math|Vector|MakeVector (.x _returnvalue) (.y _returnvalue) (+ (.z _returnvalue) 5e+01)) "0, 0, 0" "1.000000,1.000000,1.000000") "AlwaysSpawn" "MultiplyWithRoot" 0 0))

(event EventBeingHit
  (params (Damage :type Integer))
  ;[1 1 1] BeingHit
  (bind _output_get (Variables|Default|SetLife (- (Variables|Default|GetLife) Damage)))
  (if (and (<= _output_get 0) (Variables|Default|GetIsAlive))
    (Variables|Default|SetIsAlive false)
    (Animation|Montage|PlayMontage (Variables|Character|GetMesh) "/Game/Asset/Character/Enemy/Animations/AM_Death.AM_Death"
      (:OnBlendOut
        (CallFunction|DropStuff)
        (Actor|DestroyActor)))))

(event EventBeginPlay
  (for _array_element (Variables|Default|GetWeapons)
    (Components|SkinnedMesh|HideBonebyName (Variables|Character|GetMesh) _array_element "PBO_None")
    (bind _returnvalue (Game|SpawnActorfromClass (Variables|Default|GetEquipedWeapon) (Math|Transform|MakeTransform (Transformation|GetActorLocation) "0, 0, 0" "0.000000,0.000000,0.000000") "Undefined" "MultiplyWithRoot" self 0 0))
    (bind _output_get (Variables|Default|SetCurrentWeapon _returnvalue))
    (Components|SkinnedMesh|UnHideBonebyName (Variables|Character|GetMesh) (Variables|/Game/Blueprints/Props/Weapons/BP_WeaponMaster.BP_WeaponMaster_C|GetName _output_get))))

(fn ConstructionScript)