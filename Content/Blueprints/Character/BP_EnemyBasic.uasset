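; Basic enemy character that roams the level and attacks the player on sight, driven by event-graph logic.
; AI Perception updates track player visibility and last seen location, re-triggering the Roam decision event.
; Roam, gated on being alive, moves within weapon-scaled range of a visible player and fires, or investigates the last seen location.
; Otherwise it moves to random reachable nearby points, pausing briefly between moves.
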(event OnTargetPerceptionInfoUpdated(AIPerception)
  (params (UpdateInfo :type Actor%20Perception%20Update%20Info%20Structure%20%28by%20ref%29))
  ;[1 1 1] Can see player
  (if (== (.target UpdateInfo) (Game|GetPlayerCharacter 0))
    (Variables|Default|SetCanSeePlayer (.bsuccessfullysensed (.stimulus UpdateInfo)))
    (CallFunction|Roam)
    (if (not (Variables|Default|GetCanSeePlayer))
      (Variables|Default|SetLastSeenPlayerLocation (.stimuluslocation (.stimulus UpdateInfo))))))

(event Custom|Roam
  ;[1 1 1] Roam
  (if (Variables|Default|GetIsAlive)
    (if (Variables|Default|GetCanSeePlayer)
      (AI|AIMoveTo self "0, 0, 0" (Game|GetPlayerCharacter 0) (Math|Conversions|ToFloat(Integer) (* (Variables|/Game/Blueprints/Props/Weapons/BP_WeaponMaster.BP_WeaponMaster_C|GetRange (Variables|Default|GetCurrentWeapon)) 80)) true
        (:OnSuccess
          (if (Variables|Default|GetCanSeePlayer)
            (CallFunction|Fire))))
      (elif (not (Utilities|Operators|EqualEqual :A (Variables|Default|GetLastSeenPlayerLocation)))
        (AI|AIMoveTo self (Variables|Default|GetLastSeenPlayerLocation) 0 1e+01 true
          (:OnSuccess
            _)
          (:OnFail
            _))
        (CallFunction|Roam)
        (Variables|Default|SetLastSeenPlayerLocation "0, 0, 0")
        (else
          (CallFunction|RandomRoamInsidetheLevel))))))

(event Custom|FindRandomDestination
  ;[1 1 1] Get a random reachable point to go
  (Variables|Default|SetRandomLocationDestination (.RandomLocation (AI|Navigation|GetRandomReachablePointinRadius (Transformation|GetActorLocation) 1e+03 0 0))))

(event Custom|RandomRoamInsideTheLevel
  ;[1 1 1] Move arround the level
  (CallFunction|FindRandomDestination)
  (AI|AIMoveTo self (Variables|Default|GetRandomLocationDestination) 0 1e+01 true
    (:OnSuccess
      _)
    (:OnFail
      _))
  (Utilities|FlowControl|Delay (Math|Random|RandomFloatinRange 2.0 4.0))
  (CallFunction|Roam))

(event EventBeginPlay
  (|CallParentFunction)
  (CallFunction|Roam))

(fn ConstructionScript
  (|CallParentFunction))