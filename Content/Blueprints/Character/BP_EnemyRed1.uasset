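; Enemy character that wanders the level, hunts the player and shoots with its equipped weapon.
; BeginPlay spawns the weapon actor and unhides the matching mesh bone after hiding all weapon bones.
; AI Perception re-triggers Roam, an event-driven loop choosing between chase-and-fire, last seen location or random reachable points, without a behavior tree.
; BP_ClassicBullet overlaps reduce Life; death plays a montage, then destroys the actor on blend out.
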(event OnComponentBeginOverlap(CapsuleComponent)
  (params (OverlappedComponent :type Primitive%20Component%20Object%20Reference) (OtherActor :type Actor%20Object%20Reference) (OtherComp :type Primitive%20Component%20Object%20Reference) (OtherBodyIndex :type Integer) (bFromSweep :type Boolean) (SweepResult :type Hit%20Result%20Structure%20%28by%20ref%29))
  ;[1 1 1] BulletHit
  (bind _asbp_classic_bullet (Utilities|Casting|CastToBP_ClassicBullet OtherActor))
  (CallFunction|Damage (Variables|/Game/Blueprints/Props/Munitions/BP_ClassicBullet.BP_ClassicBullet_C|GetDamage _asbp_classic_bullet))
  (Actor|DestroyActor _asbp_classic_bullet))

(event OnTargetPerceptionInfoUpdated(AIPerception)
  (params (UpdateInfo :type Actor%20Perception%20Update%20Info%20Structure%20%28by%20ref%29))
  ;[1 1 1] Ai perception - can see player?
  (if (== (.target UpdateInfo) (Game|GetPlayerCharacter 0))
    (Variables|Default|SetCanSeePlayer? (.bsuccessfullysensed (.stimulus UpdateInfo)))
    (CallFunction|Roam)
    (if (not (Variables|Default|GetCanSeePlayer?))
      (Variables|Default|SetLastSeenPlayerLocation (.stimuluslocation (.stimulus UpdateInfo))))))

(event Custom|Roam
  ;[1 1 1] Roam
  (if (Variables|Default|GetIsAlive)
    (if (Variables|Default|GetCanSeePlayer?)
      (AI|AIMoveTo self "0, 0, 0" (Game|GetPlayerCharacter 0) (Variables|Default|GetMaxShootRange) true
        (:OnSuccess
          (if (Variables|Default|GetCanSeePlayer?)
            (CallFunction|Fire))))
      (elif (not (Utilities|Operators|EqualEqual :A (Variables|Default|GetLastSeenPlayerLocation)))
        (AI|AIMoveTo self (Variables|Default|GetLastSeenPlayerLocation) 0 5.0 true
          (:OnSuccess
            (CallFunction|Roam)
            (Variables|Default|SetLastSeenPlayerLocation "0, 0, 0")))
        (else
          (CallFunction|RandomRoamInsidetheLevel))))))

(event Custom|Fire
  ;[1 1 1] Fire
  (Default|Fire (Variables|Default|GetCurrentWeapon) (Transformation|GetSocketLocation (Variables|Character|GetMesh) (Variables|/Game/Blueprints/Props/Weapons/BP_WeaponMaster.BP_WeaponMaster_C|GetName (Variables|Default|GetCurrentWeapon))) (Math|Rotator|FindLookatRotation (Transformation|GetActorLocation) (Transformation|GetActorLocation (Game|GetPlayerCharacter 0))))
  (Utilities|FlowControl|Delay (Variables|Default|GetCooldDownAfterFiring))
  (CallFunction|Roam))

(event Custom|FindRandomDest
  ;[1 1 1] Get a random reachable point to go
  (Variables|Default|SetRandomLocationDest (.RandomLocation (AI|Navigation|GetRandomReachablePointinRadius (Transformation|GetActorLocation) 1e+03 0 0))))

(event Custom|RandomRoamInsideTheLevel
  ;[1 1 1] Move arround the level
  (CallFunction|FindRandomDest)
  (AI|AIMoveTo self (Variables|Default|GetRandomLocationDest) 0 5.0 true
    (:OnSuccess
      (Utilities|FlowControl|Delay (Math|Random|RandomFloatinRange 2.0 4.0))
      (CallFunction|Roam))))

(event Custom|Damage
  (params (DamageNumber :type Integer))
  ;[1 1 1] Damage
  (bind _output_get (Variables|Default|SetLife (- (Variables|Default|GetLife) DamageNumber)))
  (if (and (<= _output_get 0) (Variables|Default|GetIsAlive))
    (Variables|Default|SetIsAlive false)
    (Animation|Montage|PlayMontage (Variables|Character|GetMesh) "/Game/Asset/Character/Enemy/Animations/AM_Death.AM_Death"
      (:OnBlendOut
        (Actor|DestroyActor)))))

(event EventBeginPlay
  ;[1 1 1] BeginPlay
  (for _array_element (Variables|Default|GetWeapons)
    (Components|SkinnedMesh|HideBonebyName (Variables|Character|GetMesh) _array_element "PBO_None"))
  (bind _returnvalue (Game|SpawnActorfromClass (Variables|Default|GetEquipedWeapon) (Math|Transform|MakeTransform (Transformation|GetActorLocation) "0, 0, 0" "0.000000,0.000000,0.000000") "Undefined" "MultiplyWithRoot" self 0))
  (bind _output_get (Variables|Default|SetCurrentWeapon _returnvalue))
  (Components|SkinnedMesh|UnHideBonebyName (Variables|Character|GetMesh) (Variables|/Game/Blueprints/Props/Weapons/BP_WeaponMaster.BP_WeaponMaster_C|GetName _output_get))
  (CallFunction|Roam))

(fn ConstructionScript)