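; BP_EnemyRed2 is an enemy character that can move between waypoints, spot the player and die from bullet hits.
; BeginPlay converts waypoint offsets to world positions for FollowMoveToGo, spawns a zero-scale weapon actor and unhides only its matching mesh bone.
; PawnSensing sets a blackboard flag upon seeing BP_MainCharacter.
; Capsule overlaps with BP_ClassicBullet reduce Life, and death plays a montage before destroying the actor.
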(event OnSeePawn(PawnSensing)
  (params (Pawn :type Pawn%20Object%20Reference))
  ;[1 1 1] SeeThePlayer
  (Utilities|Casting|CastToBP_MainCharacter Pawn)
  (AI|Components|Blackboard|SetValueasBool (AI|GetBlackboard (AI|GetAIController self)) (Utilities|Name|MakeLiteralName "hasSeenPlayer?") true))

(event OnComponentBeginOverlap(CapsuleComponent)
  (params (OverlappedComponent :type Primitive%20Component%20Object%20Reference) (OtherActor :type Actor%20Object%20Reference) (OtherComp :type Primitive%20Component%20Object%20Reference) (OtherBodyIndex :type Integer) (bFromSweep :type Boolean) (SweepResult :type Hit%20Result%20Structure%20%28by%20ref%29))
  ;[1 1 1] BulletHit
  (bind _asbp_classic_bullet (Utilities|Casting|CastToBP_ClassicBullet OtherActor))
  (CallFunction|Damage (Variables|/Game/Blueprints/Props/Munitions/BP_ClassicBullet.BP_ClassicBullet_C|GetDamage _asbp_classic_bullet))
  (Actor|DestroyActor _asbp_classic_bullet))

(event Custom|Damage
  (params (DamageNumber :type Integer))
  ;[1 1 1] Damage
  (bind _output_get (Variables|Default|SetLife (- (Variables|Default|GetLife) DamageNumber)))
  (if (and (<= _output_get 0) (Variables|Default|GetIsAlive))
    (Variables|Default|SetIsAlive false)
    (Animation|Montage|PlayMontage (Variables|Character|GetMesh) "/Game/Asset/Character/Enemy/Animations/AM_Death.AM_Death"
      (:OnBlendOut
        (Actor|DestroyActor)))))

(event Custom|Follow%20MoveToGo
  (params (Nb :type Integer))
  ;[1 1 1] Round
  (AI|AIMoveTo self (Utilities|Array|Get(acopy) (Variables|Default|GetWorldMoveToGo) Nb) 0 0.0 true))

(event Custom|ConvertToWorldPo
  ;[1 1 1] ConvertToWordlPos
  (for _array_element (Variables|Default|GetMoveToGo)
    (Utilities|Array|Add (Variables|Default|GetWorldMoveToGo) (+ _array_element (Transformation|GetWorldLocation (Variables|Collision|GetCapsuleComponent self))))))

(event EventBeginPlay
  ;[1 1 1] BeginPlay
  (CallFunction|ConverttoWorldPo)
  (for _array_element (Variables|Default|GetWeapons)
    (Components|SkinnedMesh|HideBonebyName (Variables|Character|GetMesh) _array_element "PBO_None"))
  (bind _returnvalue (Game|SpawnActorfromClass (Variables|Default|GetEquipedWeapon) (Math|Transform|MakeTransform (Transformation|GetActorLocation) "0, 0, 0" "0.000000,0.000000,0.000000") "Undefined" "MultiplyWithRoot" self 0 0))
  (bind _output_get (Variables|Default|SetCurrentWeapon _returnvalue))
  (Components|SkinnedMesh|UnHideBonebyName (Variables|Character|GetMesh) (Variables|/Game/Blueprints/Props/Weapons/BP_WeaponMaster.BP_WeaponMaster_C|GetName _output_get)))

(fn ConstructionScript)