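; Enemy character blueprint that moves along designer-set points and reports player sightings to its AI blackboard.
; On BeginPlay it converts MoveToGo offsets into world positions relative to the capsule, and FollowMoveToGo sends the pawn to one by index.
; AI Perception updates set or clear the "hasSeenPlayer?" key for player zero.
; The PawnSensing sight event is empty, with its similar blackboard logic left disconnected.
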(event OnSeePawn(PawnSensing)
  (params (Pawn :type Pawn%20Object%20Reference)))

(event OnTargetPerceptionInfoUpdated(AIPerception)
  (params (UpdateInfo :type Actor%20Perception%20Update%20Info%20Structure%20%28by%20ref%29))
  ;[1 1 1] Perception Update
  (if (== (.target UpdateInfo) (Game|GetPlayerCharacter 0))
    (AI|Components|Blackboard|SetValueasBool (AI|GetBlackboard (AI|GetAIController self)) (Utilities|Name|MakeLiteralName "hasSeenPlayer?") (.bsuccessfullysensed (.stimulus UpdateInfo)))))

(event Custom|FollowMoveToGo
  (params (nb :type Integer))
  ;[1 1 1] FollowMoveToGo
  (AI|AIMoveTo self (Utilities|Array|Get(acopy) (Variables|Default|GetWorldMoveToGo) nb) 0 5.0 false))

(event Custom|ConvertToWorldPosition
  ;[1 1 1] Convert to world Position
  (for _array_element (Variables|Default|GetMoveToGo)
    (Utilities|Array|Add (Variables|Default|GetWorldMoveToGo) (+ _array_element (Transformation|GetWorldLocation (Variables|Default|GetCapsuleComponent self))))))

(event EventBeginPlay
  (|CallParentFunction)
  (CallFunction|ConverttoWorldPosition))

(fn ConstructionScript
  (|CallParentFunction))