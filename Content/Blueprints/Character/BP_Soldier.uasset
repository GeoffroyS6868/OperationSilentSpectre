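; BP_Soldier is an AI enemy that roams the level and shoots at the player, driven by event graph logic.
; AI Perception updates CanSeePlayer and LastSeenPlayerLocation, then re-runs Roam, the central decision event.
; Roam moves into shooting range and fires, investigates the last seen location, or wanders to random reachable points.
; Fire spawns a BP_Bullet aimed at the player, then returns to Roam after a cooldown.
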(event OnTargetPerceptionInfoUpdated(AIPerception)
  (params (UpdateInfo :type Actor%20Perception%20Update%20Info%20Structure%20%28by%20ref%29))
  ;[1 1 1] Ai perception - can see player?
  (if (== (.target UpdateInfo) (Game|GetPlayerCharacter 0))
    (Variables|Default|SetCanSeePlayer? (.bsuccessfullysensed (.stimulus UpdateInfo)))
    (CallFunction|Roam)
    (if (not (Variables|Default|GetCanSeePlayer?))
      (Variables|Default|SetLastSeenPlayerLocation (.stimuluslocation (.stimulus UpdateInfo))))))

(event Custom|Roam
  (if (Variables|Default|GetCanSeePlayer?)
    (AI|AIMoveTo self "0, 0, 0" (Game|GetPlayerCharacter 0) (Variables|Default|GetMaxShootRange) true
      (:OnSuccess
        (if (Variables|Default|GetCanSeePlayer?)
          (CallFunction|Fire))))
    (elif (not (Utilities|Operators|EqualEqual :A (Variables|Default|GetLastSeenPlayerLocation)))
      (AI|AIMoveTo self (Variables|Default|GetLastSeenPlayerLocation) 0 5.0 true
        (:OnSuccess
          (CallFunction|Roam)
          (Variables|Default|SetLastSeenPlayerLocation "0, 0, 0")))
      (else
        (CallFunction|RandomRoamInsidetheLevel)))))

(event Custom|Fire
  ;[1 1 1] Fire - Spawn a bullet to the our SpawnBullTransform - Get the correct rotation to fire the bullets to the player
  (Game|SpawnActorfromClass "/Game/Blueprints/Bullets/BP_Bullet.BP_Bullet_C" (Math|Transform|MakeTransform (+ (.location (Transformation|GetWorldTransform (Variables|Default|GetBulletSpawnTransform))) (Math|Vector|GetForwardVector (Math|Rotator|MakeRotator 0.0 0.0 (.Yaw (Math|Rotator|BreakRotator (Pawn|GetControlRotation :!class /Script/Engine.Pawn)))))) (Math|Rotator|FindLookatRotation (Transformation|GetActorLocation) (Transformation|GetActorLocation (Game|GetPlayerCharacter 0)))) "Undefined" "MultiplyWithRoot" 0 0)
  ;;[1 1 1] CD before AI can do something else
  (Utilities|FlowControl|Delay (Variables|Default|GetCooldDownAfterFiring))
  (CallFunction|Roam))

(event Custom|FindRandomDest
  ;[1 1 1] Get a random reachable point to go
  (Variables|Default|SetRandomLocationDest (.RandomLocation (AI|Navigation|GetRandomReachablePointinRadius (Transformation|GetActorLocation) 1.23e+03 0 0))))

(event Custom|RandomRoamInsideTheLevel
  ;[1 1 1] Move arround the level
  (CallFunction|FindRandomDest)
  (AI|AIMoveTo self (Variables|Default|GetRandomLocationDest) 0 5.0 true
    (:OnSuccess
      (Utilities|FlowControl|Delay (Math|Random|RandomFloatinRange 2.0 4.0))
      (CallFunction|Roam))))

(event EventBeginPlay
  (CallFunction|Roam)
  (for _array_element (Variables|Default|GetWeapons)
    (Components|SkinnedMesh|HideBonebyName (Variables|Character|GetMesh) _array_element "PBO_None")))

(fn ConstructionScript)