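; BP_SilentSpectreInstance, likely the game instance by its name, tracks the current and unlocked levels and handles level completion.
; FinishedLevel switches on CurrentLevel: finishing Desert Village for the first time adds Beach to AvailableLevels, clears all widgets and shows the win menu with cursor and UI-only input.
; The win menu appears only on that first unlock, and Beach has no completion logic.
; GetCurrentLevelName maps the level enum to its name string.
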(fn FinishedLevel
  (bind _returnvalue (Game|GetPlayerController 0))
  (switch Utilities|FlowControl|Switch|SwitchonE_Levels (Variables|Default|GetCurrentLevel)
    (:NewEnumerator0
      (if (== (Utilities|Array|FindItem (Variables|Default|GetAvailableLevels) "NewEnumerator1") -1)
        (Utilities|Array|Add (Variables|Default|GetAvailableLevels) "NewEnumerator1")
        (Viewport|RemoveAllWidgets)
        (bind _returnvalue_2 (UserInterface|CreateWidget "/Game/Blueprints/Widget/WBP_WinMenu.WBP_WinMenu_C" _returnvalue))
        (Variables|/Script/Engine.PlayerController|SetbShowMouseCursor _returnvalue true)
        (Input|SetInputModeUIOnly _returnvalue _returnvalue_2 "DoNotLock" false)
        (UserInterface|Viewport|AddtoViewport _returnvalue_2 0)))))

(fn GetCurrentLevelName
  (switch Utilities|FlowControl|Switch|SwitchonE_Levels (Variables|Default|GetCurrentLevel)
    (:NewEnumerator0
      (return "DesertVillage"))
    (:NewEnumerator1
      (return "Beach"))))