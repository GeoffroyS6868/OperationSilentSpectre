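; Multiplayer game state that runs a ten-minute match timer once the minimum player count connects.
; The MatchTimeCountdown RepNotify updates HUD widgets and, on authority, re-triggers a one-second delayed decrement, forming a self-driven loop.
; At zero, finish-screen RPC events reveal scoreboards, then after a delay destroy the session and open the main menu, whether or not destruction succeeds.
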(event Custom|UpdatePlayerConnection
  ;[0.04688 0.04688 0.04688] Update Player Connection
  (if (>= (Class|GameplayStatics|GetNumPlayerStates) (Variables|Default|GetMinimumRequiredPlayer))
    (Utilities|FlowControl|DoOnce false
      (:Completed
        (Variables|Default|SetMatchTimeCountdown 600)))))

(event Custom|MatchCountdown
  ;[0.04271 0.04271 0.04271] Match Count Down
  (Utilities|FlowControl|Delay 1.0)
  (Variables|Default|SetMatchTimeCountdown (- (Variables|Default|GetMatchTimeCountdown) 1)))

(event Custom|RPC_FinishScreen
  ;[0.04688 0.04688 0.04688] FinishScreen
  (bind _foundwidgets (Widget|GetAllWidgetsOfClass "/Game/Blueprints/Widget/Multiplayer/WBP_ScoreBoard.WBP_ScoreBoard_C" false))
  (for _array_element _foundwidgets
    (Widget|SetVisibility _array_element "Visible"))
  (CallFunction|Quit))

(event Custom|RPC_Server_FinishScreen
  (CallFunction|RPCFinishScreen))

(event Custom|Quit
  ;[0.04688 0.04688 0.04688] Quit
  (Utilities|FlowControl|Delay 1e+01)
  (|DestroySession
    (:OnSuccess
      _)
    (:OnFailure
      _))
  (Game|OpenLevel(byName) "MainMenu"))

(fn ConstructionScript)

(fn OnRepMatchTimeCountdown
  (CallFunction|UpdateMatchCountDownWidget)
  (Networking|SwitchHasAuthority
    (:Authority
      (if (== (Variables|Default|GetMatchTimeCountdown) 600)
        (CallFunction|MatchCountdown)
        (elif (<= (Variables|Default|GetMatchTimeCountdown) 0)
          (CallFunction|RPCServerFinishScreen)
          (else
            (CallFunction|MatchCountdown)))))))

(fn UpdateMatchCountDownWidget
  (bind _foundwidgets (Widget|GetAllWidgetsOfClass "/Game/Blueprints/Widget/Multiplayer/WBP_MultiplayerHud.WBP_MultiplayerHud_C" false))
  (for _array_element _foundwidgets
    (Default|UpdateCountDown _array_element (Variables|Default|GetMatchTimeCountdown))))