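; BP_RocketBullet is a rocket projectile actor that explodes on contact.
; On BeginPlay it starts a timer derived from Range and destroys itself without exploding when that runs out.
; When CollisionComponent begins an overlap, it removes that component, spawns BP_Explosion at the sweep impact point and destroys itself.
; The collision location saved in PosToSpawnExplosion is not used for the spawn.
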(event OnComponentBeginOverlap(CollisionComponent)
  (params (OverlappedComponent :type Primitive%20Component%20Object%20Reference) (OtherActor :type Actor%20Object%20Reference) (OtherComp :type Primitive%20Component%20Object%20Reference) (OtherBodyIndex :type Integer) (bFromSweep :type Boolean) (SweepResult :type Hit%20Result%20Structure%20%28by%20ref%29))
  (Variables|Default|SetPosToSpawnExplosion (Transformation|GetWorldLocation (Variables|MyProjectile|GetCollisionComponent)))
  (Components|DestroyComponent (Variables|MyProjectile|GetCollisionComponent))
  (Game|SpawnActorfromClass "/Game/Blueprints/Props/BP_Explosion.BP_Explosion_C" (Math|Transform|MakeTransform (.impactpoint SweepResult) "0, 0, 0" "1.000000,1.000000,1.000000") "AlwaysSpawn" "MultiplyWithRoot" 0 0)
  (Actor|DestroyActor))

(event EventBeginPlay
  (Utilities|FlowControl|Delay (/ (Math|Conversions|ToFloat(Integer) (Variables|Default|GetRange)) 1e+01))
  (Actor|DestroyActor))

(fn ConstructionScript)