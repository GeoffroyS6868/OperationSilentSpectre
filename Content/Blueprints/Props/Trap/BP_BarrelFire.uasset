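; Fire barrel trap prop that ignites when hit and then damages overlapping actors until it destroys itself.
; BeingHit lights it once, adding three Niagara effects, setting the trigger box extent, playing a fire sound and starting a timed self-destruct.
; While lit, an overlap sends BeingHitMessage to BPI_BeingHit actors.
; The box is briefly teleported away and back to its saved position, so lingering actors are hit repeatedly.
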(event OnComponentBeginOverlap(Box)
  (params (OverlappedComponent :type Primitive%20Component%20Object%20Reference) (OtherActor :type Actor%20Object%20Reference) (OtherComp :type Primitive%20Component%20Object%20Reference) (OtherBodyIndex :type Integer) (bFromSweep :type Boolean) (SweepResult :type Hit%20Result%20Structure%20%28by%20ref%29))
  (bind _box (Variables|Default|GetBox))
  ;[0.04688 0.04688 0.04688] OverlapFire
  (if (Variables|Default|Getonfire)
    (if (Utilities|DoesObjectImplementInterface OtherActor "/Game/Blueprints/Core/Interface/BPI_BeingHit.BPI_BeingHit_C")
      (Class|BPIBeingHit|BeingHit(Message) OtherActor 10)
      (Transformation|SetWorldLocation _box "-1000.000000,-1000.000000,-1000.000000" false false)
      (Utilities|FlowControl|Delay 1.0)
      (Transformation|SetWorldLocation _box (Variables|Default|Getplace) false false))))

(event EventBeginPlay
  (Variables|Default|Setplace (Transformation|GetWorldLocation (Variables|Default|GetBox))))

(event EventBeingHit
  (params (Damage :type Integer))
  ;[0.04271 0.04271 0.04271] ActivateFire
  (if (not (Variables|Default|Getonfire))
    (Variables|Default|Setonfire true)
    (bind _returnvalue (AddComponent|AddNiagaraComponent false))
    (Transformation|SetRelativeLocation _returnvalue (Variables|/Script/Engine.SceneComponent|GetRelativeLocation (Variables|Default|Getrw)) false false)
    (bind _returnvalue_2 (AddComponent|AddNiagaraComponent false))
    (Transformation|SetRelativeLocation _returnvalue_2 (Variables|/Script/Engine.SceneComponent|GetRelativeLocation (Variables|Default|Getrw4)) false false)
    (bind _returnvalue_3 (AddComponent|AddNiagaraComponent false))
    (Transformation|SetRelativeLocation _returnvalue_3 (Variables|/Script/Engine.SceneComponent|GetRelativeLocation (Variables|Default|Getrw8)) false false)
    (Components|Box|SetBoxExtent (Variables|Default|GetBox) "32.000000,32.000000,32.000000" true)
    (Audio|SpawnSoundatLocation "/Game/Asset/Audio/Sounds/Trap/Fire.Fire" (Transformation|GetActorLocation) "0, 0, 0" 1.0 1.0 0.0 "/Game/Asset/Audio/SA_Main.SA_Main" 0)
    (Utilities|FlowControl|Delay 1e+01)
    (Actor|DestroyActor)))

(fn ConstructionScript)