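; Barrel trap prop that ignites when hit by a BP_ClassicBullet, then burns enemies that touch it.
; On ignition it destroys the bullet, sets Onfire, adds a Niagara fire effect and destroys itself after a delay.
; While burning, overlapping BP_EnemyRed1 actors take damage, then after a short delay the box collapses and restores its extent to retrigger overlap for repeated damage.
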(event OnComponentBeginOverlap(Box)
  (params (OverlappedComponent :type Primitive%20Component%20Object%20Reference) (OtherActor :type Actor%20Object%20Reference) (OtherComp :type Primitive%20Component%20Object%20Reference) (OtherBodyIndex :type Integer) (bFromSweep :type Boolean) (SweepResult :type Hit%20Result%20Structure%20%28by%20ref%29))
  (bind _box (Variables|Default|GetBox))
  (if (Variables|Default|Getonfire)
    (bind _asbp_enemy_red_1 (Utilities|Casting|CastToBP_EnemyRed1 OtherActor))
    (Default|Damage _asbp_enemy_red_1 10)
    (Development|PrintText "ooch")
    (Utilities|FlowControl|Delay 1.0)
    (Components|Box|SetBoxExtent _box "0.000000,0.000000,0.000000" true)
    (Components|Box|SetBoxExtent _box "32.000000,32.000000,32.000000" true)
    (else
      (bind _asbp_classic_bullet (Utilities|Casting|CastToBP_ClassicBullet OtherActor))
      (Actor|DestroyActor _asbp_classic_bullet)
      (Variables|Default|Setonfire true)
      (bind _returnvalue (AddComponent|AddNiagaraComponent false))
      (Variables|Default|Setfire _returnvalue)
      (Components|Box|SetBoxExtent (Variables|Default|GetBox) "32.000000,32.000000,32.000000" true)
      (Utilities|FlowControl|Delay 1e+01)
      (Actor|DestroyActor))))

(event EventBeginPlay)

(event Collision|EventActorBeginOverlap
  (params (OtherActor :type Actor%20Object%20Reference)))

(event EventTick
  (params (DeltaSeconds :type Float%20%28single-precision%29)))

(fn ConstructionScript)