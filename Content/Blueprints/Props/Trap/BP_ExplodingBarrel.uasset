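; Exploding barrel trap prop that, when hit, burns for three seconds and then explodes.
; BeingHit runs a delayed sequence: fire effect, then explosion effect and sound with the barrel mesh and box removed, then actor destruction.
; The blast works by enlarging a sphere so its begin-overlap event sends a BeingHit message with 100 to actors implementing BPI_BeingHit.
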(event OnComponentBeginOverlap(explosionsphere)
  (params (OverlappedComponent :type Primitive%20Component%20Object%20Reference) (OtherActor :type Actor%20Object%20Reference) (OtherComp :type Primitive%20Component%20Object%20Reference) (OtherBodyIndex :type Integer) (bFromSweep :type Boolean) (SweepResult :type Hit%20Result%20Structure%20%28by%20ref%29))
  ;[1 1 1] Explosion Sphere
  (if (Utilities|DoesObjectImplementInterface OtherActor "/Game/Blueprints/Core/Interface/BPI_BeingHit.BPI_BeingHit_C")
    (Class|BPIBeingHit|BeingHit(Message) OtherActor 100)))

(event EventBeingHit
  (params (Damage :type Integer))
  ;[1 1 1] BeingHit
  (bind _returnvalue (AddComponent|AddNiagaraComponent false))
  (bind _output_get (Variables|Default|Setfire_temp _returnvalue))
  (Utilities|FlowControl|Delay 3.0)
  (Components|DestroyComponent _output_get)
  (bind _returnvalue_2 (AddComponent|AddNiagaraComponent false))
  (Variables|Default|SetExlosion _returnvalue_2)
  (Components|DestroyComponent (Variables|Default|GetBox))
  (Components|DestroyComponent (Variables|Default|GetExplodingBarrel))
  (Components|Sphere|SetSphereRadius (Variables|Default|Getexplosionsphere) 3e+02 true)
  (Audio|PlaySoundatLocation "/Game/Asset/Audio/Sounds/Trap/BarrelExplosion.BarrelExplosion" (Transformation|GetActorLocation) "0, 0, 0" 1.0 1.0 0.0 "/Game/Asset/Audio/SA_Main.SA_Main" 0 0 0)
  (Utilities|FlowControl|Delay 1.0)
  (Actor|DestroyActor))

(fn ConstructionScript)