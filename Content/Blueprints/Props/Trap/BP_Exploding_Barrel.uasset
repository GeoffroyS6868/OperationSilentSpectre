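; BP_Exploding_Barrel is a trap prop that explodes when a BP_ClassicBullet overlaps its box.
; The hit destroys the bullet, adds a Niagara explosion effect and removes the box and barrel components.
; It then enlarges the Explosionsphere with overlap updates, so its begin-overlap event damages BP_EnemyRed1 actors in range.
; The barrel actor destroys itself after a short delay.
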(event OnComponentBeginOverlap(Box)
  (params (OverlappedComponent :type Primitive%20Component%20Object%20Reference) (OtherActor :type Actor%20Object%20Reference) (OtherComp :type Primitive%20Component%20Object%20Reference) (OtherBodyIndex :type Integer) (bFromSweep :type Boolean) (SweepResult :type Hit%20Result%20Structure%20%28by%20ref%29))
  (bind _asbp_classic_bullet (Utilities|Casting|CastToBP_ClassicBullet OtherActor))
  (Actor|DestroyActor _asbp_classic_bullet)
  (bind _returnvalue (AddComponent|AddNiagaraComponent false))
  (Variables|Default|Setexlosion _returnvalue)
  (Components|DestroyComponent (Variables|Default|GetBox))
  (Components|DestroyComponent (Variables|Default|GetExplodingBarrel))
  (Components|Sphere|SetSphereRadius (Variables|Default|Getexplosionsphere) 3e+02 true)
  (Utilities|FlowControl|Delay 1.0)
  (Actor|DestroyActor))

(event OnComponentBeginOverlap(explosionsphere)
  (params (OverlappedComponent :type Primitive%20Component%20Object%20Reference) (OtherActor :type Actor%20Object%20Reference) (OtherComp :type Primitive%20Component%20Object%20Reference) (OtherBodyIndex :type Integer) (bFromSweep :type Boolean) (SweepResult :type Hit%20Result%20Structure%20%28by%20ref%29))
  (bind _asbp_enemy_red_1 (Utilities|Casting|CastToBP_EnemyRed1 OtherActor))
  (Default|Damage _asbp_enemy_red_1 100))

(fn ConstructionScript)