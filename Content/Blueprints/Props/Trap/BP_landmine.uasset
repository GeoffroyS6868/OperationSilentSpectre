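; BP_landmine is a trap prop that explodes when BP_MainCharacter overlaps its Box trigger.
; The trigger spawns a Niagara effect, plays the explosion sound, removes the box and mine components, then expands the Sphere into a blast radius.
; Sphere overlaps send heavy damage through BPI_BeingHit and destroy the actor immediately; otherwise it is destroyed after a short delay.
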(event OnComponentBeginOverlap(Sphere)
  (params (OverlappedComponent :type Primitive%20Component%20Object%20Reference) (OtherActor :type Actor%20Object%20Reference) (OtherComp :type Primitive%20Component%20Object%20Reference) (OtherBodyIndex :type Integer) (bFromSweep :type Boolean) (SweepResult :type Hit%20Result%20Structure%20%28by%20ref%29))
  (if (Utilities|DoesObjectImplementInterface OtherActor "/Game/Blueprints/Core/Interface/BPI_BeingHit.BPI_BeingHit_C")
    (Class|BPIBeingHit|BeingHit(Message) OtherActor 100)
    (Actor|DestroyActor)))

(event OnComponentBeginOverlap(Box)
  (params (OverlappedComponent :type Primitive%20Component%20Object%20Reference) (OtherActor :type Actor%20Object%20Reference) (OtherComp :type Primitive%20Component%20Object%20Reference) (OtherBodyIndex :type Integer) (bFromSweep :type Boolean) (SweepResult :type Hit%20Result%20Structure%20%28by%20ref%29))
  (Utilities|Casting|CastToBP_MainCharacter OtherActor)
  (bind _returnvalue (AddComponent|AddNiagaraComponent false))
  (Variables|Default|SetExplosion _returnvalue)
  (Audio|PlaySoundatLocation "/Game/Asset/Audio/Sounds/Trap/MineExplosion.MineExplosion" (Transformation|GetActorLocation) "0, 0, 0" 1.0 1.0 0.0 "/Game/Asset/Audio/SA_Main.SA_Main" 0 0 0)
  (Components|DestroyComponent (Variables|Default|GetBox))
  (Components|DestroyComponent (Variables|Default|GetLandmine))
  (Components|Sphere|SetSphereRadius (Variables|Default|GetSphere) 3e+02 true)
  (Utilities|FlowControl|Delay 1.0)
  (Actor|DestroyActor))

(fn ConstructionScript)