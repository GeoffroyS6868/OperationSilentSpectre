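; Rocket launcher weapon Blueprint that fires rocket projectile actors.
; Fire does nothing while reloading, checks ammo, and applies the fire-rate check only when CanSpam is set.
; Each shot decrements and broadcasts magazine ammo, then spawns BP_RocketBullet with Damage and Range, offset forward from the computed spawn transform.
; It also plays a shoot montage on an owning BP_MainCharacter and reuses the GlockShoot sound.
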(event EventBeginPlay
  (|CallParentFunction) ; This node is disabled and will not be called.\nDrag off pins to build functionality.
)

(event Collision|EventActorBeginOverlap
  (params (OtherActor :type Actor%20Object%20Reference)))

(event EventTick
  (params (DeltaSeconds :type Float%20%28single-precision%29)))

(fn ConstructionScript
  (|CallParentFunction))

(fn Fire
  (params (WeaponLocation :type Vector :default "0, 0, 0") (Rotator :type Rotator :default "0, 0, 0") (PlayerLocation :type Vector :default "0, 0, 0"))
  (if (not (Variables|Default|GetIsReloading))
    (if (Variables|Default|GetCanSpam)
      (bind _canfire (CallFunction|HandleFireRate))
      (bind _ammo (CallFunction|HasAmmo))
      (if (and _ammo _canfire)
        (bind _result (Math|Integer|DecrementInt (Variables|Default|GetCurrentMagazine) :!label _label)
          (:%20%20
            (Default|CallCurrentMagazineAmmoUpdated _result)
            (bind _bullettransform (CallFunction|GetSpawnTransform WeaponLocation Rotator))
            (Game|SpawnActorfromClass "/Game/Blueprints/Props/Munitions/BP_RocketBullet.BP_RocketBullet_C" (Math|Transform|MakeTransform (+ (.location _bullettransform) (Math|Vector|RotateVector (Math|Vector|MakeVector 3e+02 0.0 0.0) (.rotation _bullettransform))) (.rotation _bullettransform) (.scale _bullettransform)) "Undefined" "MultiplyWithRoot" 0 (Variables|Default|GetDamage) (Variables|Default|GetRange) 0)
            (bind _asbp_main_character (Utilities|Casting|CastToBP_MainCharacter (Components|GetOwner))
              (:then
                (Animation|Montage|MontagePlay (Components|SkeletalMesh|GetAnimInstance (Variables|/Game/Blueprints/Character/BP_MainCharacter.BP_MainCharacter_C|GetSkeletalMesh _asbp_main_character)) "/Game/Animations/AM_Shoot.AM_Shoot" 1.0 "MontageLength" 0.0 true))
              (:CastFailed
                _))
            (Audio|PlaySoundatLocation "/Game/Asset/Audio/Sounds/Weapons/Glock/GlockShoot.GlockShoot" WeaponLocation "0, 0, 0" 1.0 1.0 0.0 0 0 0 0))))
      (else
        (bind _ammo_2 (CallFunction|HasAmmo))
        (if _ammo_2
          (goto _label))))))