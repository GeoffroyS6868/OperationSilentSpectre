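; Sniper rifle weapon Blueprint that adds a toggleable scope and its own sounds to a parent class.
; UseSecondary flips IsScoping, calls CallSniperScope, hides or restores the character's Sniper bone, changes the first-person camera's aspect ratio, then notifies MainCharacter of the new state.
; Fire audio plays at the given location, while reload audio plays as 2D sound and ignores its Location input.
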(event EventBeginPlay
  (|CallParentFunction))

(fn ConstructionScript
  (|CallParentFunction))

(fn UseSecondary
  (bind _maincharacter (Variables|Default|GetMainCharacter))
  (bind _skeletalmesh (Variables|/Game/Blueprints/Character/BP_MainCharacter.BP_MainCharacter_C|GetSkeletalMesh _maincharacter))
  (bind _firstpersoncamera (Variables|/Game/Blueprints/Character/BP_MainCharacter.BP_MainCharacter_C|GetFirstPersonCamera _maincharacter))
  (Variables|Default|SetIsScoping (not (Variables|Default|GetIsScoping)))
  (Utilities|FlowControl|Sequence
    (:then_0
      (Default|CallSniperScope))
    (:then_1
      (if (Variables|Default|GetIsScoping)
        (Components|SkinnedMesh|HideBonebyName _skeletalmesh "Sniper" "PBO_None")
        (Class|CameraComponent|SetAspectRatio _firstpersoncamera 5.0)
        (else
          (Components|SkinnedMesh|UnHideBonebyName _skeletalmesh "Sniper")
          (Class|CameraComponent|SetAspectRatio _firstpersoncamera (Math|Float|SafeDivide 16.0 9.0)))))
    (:then_2
      (Default|ScopingUpdated _maincharacter (Variables|Default|GetIsScoping)))))

(fn PlayFireSound
  (params (Location :type Vector :default "0, 0, 0"))
  (Audio|PlaySoundatLocation "/Game/Asset/Audio/Sounds/Weapons/Sniper/SniperShoot.SniperShoot" Location "0, 0, 0" 1.0 1.0 0.0 0 0 0 0))

(fn PlayReloadSound
  (params (Location :type Vector :default "0, 0, 0"))
  (Audio|PlaySound2D "/Game/Asset/Audio/Sounds/Weapons/Sniper/SniperReload.SniperReload" 1.0 1.0 0.0 0 0))