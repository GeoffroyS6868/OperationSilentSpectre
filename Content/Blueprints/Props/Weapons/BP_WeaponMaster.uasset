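; Base weapon for hitscan guns, handling firing, magazine ammo and timed reloads from the owning BP_MainCharacter's reserves.
; Shoot line-traces with spread that grows over quick successive shots and shrinks with Precision, gated by FireRate.
; Hits send damage through BPI_BeingHit or leave random impact decals, and magazine changes are broadcast.
; Sounds route through the owner's BPI_PlaySound, else play at location, with gunfire also emitting noise; UseSecondary is an empty stub.
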(event Custom|Shoot
  (params (Rotator :type Rotator) (OwnerLocation :type Vector))
  ;[0.05104 0.05104 0.05104] Shoot
  (if (not (Variables|Default|GetIsReloading))
    (bind _ammo (CallFunction|HasAmmo))
    (if _ammo
      (if (Variables|Default|GetCanShoot)
        (Variables|Default|SetCanShoot false)
        (bind _rotator (CallFunction|GetRandomRotation))
        (bind _result (Math|Integer|DecrementInt (Variables|Default|GetCurrentMagazine))
          (:%20%20
            (Default|CallCurrentMagazineAmmoUpdated _result)
            (bind _outhit (Collision|LineTraceByChannel OwnerLocation (+ (Math|Vector|RotateVector (Math|Vector|RotateVector (Math|Vector|MakeVector (* (Math|Conversions|ToFloat(Integer) (Variables|Default|GetRange)) 1e+02) 0.0 0.0) _rotator) Rotator) OwnerLocation) "TraceTypeQuery2" false (Utilities|Array|MakeArray (Components|GetOwner)) "ForDuration"))
            (Utilities|IsValid (.hitactor _outhit)
              (:Is%20Valid
                (if (Utilities|DoesObjectImplementInterface (.hitactor _outhit) "/Game/Blueprints/Core/Interface/BPI_BeingHit.BPI_BeingHit_C")
                  (Class|BPIBeingHit|BeingHit(Message) (.hitactor _outhit) (Variables|Default|GetDamage))
                  (else
                    (CallFunction|SpawnImpact (.hitcomponent _outhit) (.location _outhit) (.normal _outhit))))
                (bind _asbp_main_character (Utilities|Casting|CastToBP_MainCharacter (Components|GetOwner))
                  (:then
                    (Animation|Montage|MontagePlay (Components|SkeletalMesh|GetAnimInstance (Variables|/Game/Blueprints/Character/BP_MainCharacter.BP_MainCharacter_C|GetSkeletalMesh _asbp_main_character)) "/Game/Animations/AM_Shoot.AM_Shoot" 1.0 "MontageLength" 0.0 true))
                  (:CastFailed
                    _)))
              (:Is%20Not%20Valid
                _))
            (CallFunction|PlayFireSound OwnerLocation)
            (Utilities|FlowControl|Delay (Math|Float|SafeDivide 1.0 (Math|Conversions|ToFloat(Integer) (Variables|Default|GetFireRate))))
            (Variables|Default|SetCanShoot true)
            (Variables|Default|SetLastShotTime (Utilities|Time|GetTimeSeconds))))))))

(event Custom|Reload
  (params (Location :type Vector))
  (bind _maincharacter (Variables|Default|GetMainCharacter))
  (bind _ammotype (Variables|Default|GetAmmoType))
  (bind _maincharacter_2 (Variables|Default|GetMainCharacter))
  (bind _ammotype_2 (Variables|Default|GetAmmoType))
  (bind _returnvalue (Math|Conversions|ToInteger(Byte) _ammotype_2))
  (bind _ammos (Variables|/Game/Blueprints/Character/BP_MainCharacter.BP_MainCharacter_C|GetAmmos _maincharacter_2))
  (bind _output (Utilities|Array|Get(acopy) _ammos _returnvalue))
  ;[0.05104 0.05104 0.05104] Reloading
  (if (Math|Boolean|ANDBoolean (not (Variables|Default|GetIsReloading)) (!= (Variables|Default|GetCurrentMagazine) (Variables|Default|GetMagazineSize)) (!= _output 0))
    (Variables|Default|SetIsReloading true)
    (CallFunction|PlayReloadSound Location)
    (bind _output_get (Variables|Default|SetTotalAmmo _output))
    (Utilities|FlowControl|Delay (Variables|Default|GetTimeToReload))
    (if (< _output_get (- (Variables|Default|GetMagazineSize) (Variables|Default|GetCurrentMagazine)))
      (Default|RemoveAmmo _maincharacter _ammotype _output_get)
      (Variables|Default|SetCurrentMagazine (+ _output_get (Variables|Default|GetCurrentMagazine)))
      (else
        (Default|RemoveAmmo _maincharacter _ammotype (- (Variables|Default|GetMagazineSize) (Variables|Default|GetCurrentMagazine)))
        (Variables|Default|SetCurrentMagazine (+ (- (Variables|Default|GetMagazineSize) (Variables|Default|GetCurrentMagazine)) (Variables|Default|GetCurrentMagazine)))))
    (Variables|Default|SetIsReloading false)
    (Default|CallCurrentMagazineAmmoUpdated (Variables|Default|GetCurrentMagazine))))

(event EventBeginPlay
  (bind _asbp_main_character (Utilities|Casting|CastToBP_MainCharacter (Components|GetOwner)))
  (Variables|Default|SetMainCharacter _asbp_main_character))

(fn ConstructionScript)

(fn GetSpawnTransform
  (params (NodeLocation :type Vector) (CameraRotation :type Rotator))
  (return (Math|Transform|MakeTransform NodeLocation CameraRotation "0.100000,0.100000,0.100000")))

(fn HasAmmo
  (return (not (== (Variables|Default|GetCurrentMagazine) 0))))

(fn UseSecondary)

(fn PlayReloadSound
  (params (Location :type Vector))
  (bind _returnvalue (Components|GetOwner))
  (bind _reloadsound (Variables|Default|GetReloadSound))
  (if (Utilities|DoesObjectImplementInterface _returnvalue "/Game/Blueprints/Core/Interface/BPI_PlaySound.BPI_PlaySound_C")
    (Class|BPIPlaySound|PlaySound(Message) _returnvalue _reloadsound)
    (else
      (Audio|PlaySoundatLocation _reloadsound Location "0, 0, 0" 1.0 1.0 0.0 "/Game/Asset/Audio/SA_Main.SA_Main" 0 0 0))))

(fn PlayFireSound
  (params (Location :type Vector))
  (bind _returnvalue (Components|GetOwner))
  (bind _firesound (Variables|Default|GetFireSound))
  (if (Utilities|DoesObjectImplementInterface _returnvalue "/Game/Blueprints/Core/Interface/BPI_PlaySound.BPI_PlaySound_C")
    (Class|BPIPlaySound|PlaySound(Message) _returnvalue _firesound)
    (else
      (Audio|PlaySoundatLocation _firesound Location "0, 0, 0" 1.0 1.0 0.0 "/Game/Asset/Audio/SA_Main.SA_Main" 0 0 0)
      (Class|AISenseHearing|ReportNoiseEvent Location 1.0 self 5e+02 "None")
      (Class|Actor|MakeNoise 1.0 0 Location 5e+02 "None"))))

(fn SpawnImpact
  (params (OtherComp :type Primitive%20Component%20Object%20Reference) (HitLocation :type Vector) (HitNormal :type Vector))
  (bind _newparam (CallFunction|GetRandomImpactMaterial))
  (Class|GameplayStatics|SpawnDecalAttached _newparam "16.000000,32.000000,32.000000" OtherComp "None" HitLocation (Math|Rotator|MakeRotfromX HitNormal) "KeepWorldPosition" 1e+01))

(fn GetRandomImpactMaterial
  (switch int (Math|Random|RandomIntegerinRange 0 1)
    (:Default
      (return "/Game/Asset/Materials/MAT_Impact1.MAT_Impact1"))
    (:0
      (return "/Game/Asset/Materials/MAT_Impact1.MAT_Impact1"))
    (:1
      (return "/Game/Asset/Materials/MAT_Impact2.MAT_Impact2"))))

(fn GetRandomRotation
  (bind _precision (Variables|Default|GetPrecision))
  (bind _returnvalue (- 1e+02 _precision))
  (bind _returnvalue_2 (/ _returnvalue 1e+02))
  (if (< 3e+01 (* (- (Utilities|Time|GetTimeSeconds) (Variables|Default|GetLastShotTime)) 1e+02))
    (Variables|Default|SetShotStreak 1.0)
    (else
      (Math|Float|IncrementFloat (Variables|Default|GetShotStreak)
        (:%20%20
          _))))
  (return (Math|Rotator|MakeRotator 0.0 (* (Math|Random|RandomFloatinRange (* -0.5 (Variables|Default|GetShotStreak)) (* 0.5 (Variables|Default|GetShotStreak))) _returnvalue_2) (* (Math|Random|RandomFloatinRange (* -0.5 (Variables|Default|GetShotStreak)) (* 0.5 (Variables|Default|GetShotStreak))) _returnvalue_2))))