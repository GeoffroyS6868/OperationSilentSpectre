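; Base multiplayer weapon Blueprint that handles hitscan shooting, magazine ammo and timed reloading for its owning BP_MultiplayerCharacter.
; Shoot is rate-limited and line-traces along the supplied rotation, with random spread that grows over rapid shot streaks and shrinks with Precision.
; Hits notify BPI_BeingHit actors or otherwise spawn random impact decals.
; Sounds route through the owner's BPI_PlaySound interface, falling back to positional playback; UseSecondary is an empty stub.
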(event Custom|Reload
  (params (Location :type Vector))
  ;[0.05104 0.05104 0.05104] Reloading
  (if (and (not (Variables|Default|GetIsReloading)) (!= (Variables|Default|GetCurrentMagazine) (Variables|Default|GetMagazineSize)))
    (Variables|Default|SetIsReloading true)
    (CallFunction|PlayReloadSound Location)
    (Utilities|FlowControl|Delay (Variables|Default|GetTimeToReload))
    (Variables|Default|SetCurrentMagazine (Variables|Default|GetMagazineSize))
    (Variables|Default|SetIsReloading false)
    (Default|CallCurrentMagazineAmmoUpdated (Variables|Default|GetCurrentMagazine))))

(event Custom|Shoot
  (params (Rotator :type Rotator) (OwnerLocation :type Vector))
  ;[0.05104 0.05104 0.05104] Shoot
  (if (not (Variables|Default|GetIsReloading))
    (bind _ammo (CallFunction|HasAmmo))
    (if _ammo
      (if (Variables|Default|GetCanShoot)
        (Variables|Default|SetCanShoot false)
        (bind _rotator (CallFunction|GetRandomRotation))
        (bind _result (Math|Integer|DecrementInt (Variables|Default|GetCurrentMagazine))
          (:%20%20
            (Default|CallCurrentMagazineAmmoUpdated _result)
            (bind _outhit (Collision|LineTraceByChannel OwnerLocation (+ (Math|Vector|RotateVector (Math|Vector|RotateVector (Math|Vector|MakeVector (* (Math|Conversions|ToFloat(Integer) (Variables|Default|GetRange)) 1e+02) 0.0 0.0) _rotator) Rotator) OwnerLocation) "TraceTypeQuery2" false (Utilities|Array|MakeArray (Components|GetOwner)) "ForDuration"))
            (if (Utilities|DoesObjectImplementInterface (.hitactor _outhit) "/Game/Blueprints/Core/Interface/BPI_BeingHit.BPI_BeingHit_C")
              (Class|BPIBeingHit|MultiplayerBeingHit(Message) (.hitactor _outhit) (Variables|Default|GetDamage) (Variables|Default|GetPlayerOwner))
              (else
                (CallFunction|SpawnImpact (.hitcomponent _outhit) (.location _outhit) (.normal _outhit))))
            (CallFunction|PlayFireSound OwnerLocation)
            (Utilities|FlowControl|Delay (Math|Float|SafeDivide 1.0 (Math|Conversions|ToFloat(Integer) (Variables|Default|GetFireRate))))
            (Variables|Default|SetCanShoot true)
            (Variables|Default|SetLastShotTime (Utilities|Time|GetTimeSeconds))))))))

(event EventBeginPlay
  (bind _asbp_multiplayer_character (Utilities|Casting|CastToBP_MultiplayerCharacter (Components|GetOwner)))
  (Variables|Default|SetPlayerOwner _asbp_multiplayer_character))

(fn ConstructionScript)

(fn GetSpawnTransform
  (params (NodeLocation :type Vector) (CameraRotation :type Rotator))
  (return (Math|Transform|MakeTransform NodeLocation CameraRotation "0.100000,0.100000,0.100000")))

(fn HasAmmo
  (return (not (== (Variables|Default|GetCurrentMagazine) 0))))

(fn UseSecondary)

(fn PlayReloadSound
  (params (Location :type Vector))
  (bind _returnvalue (Components|GetOwner))
  (bind _reloadsound (Variables|Default|GetReloadSound))
  (if (Utilities|DoesObjectImplementInterface _returnvalue "/Game/Blueprints/Core/Interface/BPI_PlaySound.BPI_PlaySound_C")
    (Class|BPIPlaySound|PlaySound(Message) _returnvalue _reloadsound)
    (else
      (Audio|PlaySoundatLocation _reloadsound Location "0, 0, 0" 1.0 1.0 0.0 "/Game/Asset/Audio/SA_Main.SA_Main" 0 0 0))))

(fn PlayFireSound
  (params (Location :type Vector))
  (bind _returnvalue (Components|GetOwner))
  (bind _firesound (Variables|Default|GetFireSound))
  (if (Utilities|DoesObjectImplementInterface _returnvalue "/Game/Blueprints/Core/Interface/BPI_PlaySound.BPI_PlaySound_C")
    (Class|BPIPlaySound|PlaySound(Message) _returnvalue _firesound)
    (else
      (Audio|PlaySoundatLocation _firesound Location "0, 0, 0" 1.0 1.0 0.0 "/Game/Asset/Audio/SA_Main.SA_Main" 0 0 0))))

(fn SpawnImpact
  (params (OtherComp :type Primitive%20Component%20Object%20Reference) (HitLocation :type Vector) (HitNormal :type Vector))
  (bind _newparam (CallFunction|GetRandomImpactMaterial))
  (Class|GameplayStatics|SpawnDecalAttached _newparam "16.000000,32.000000,32.000000" OtherComp "None" HitLocation (Math|Rotator|MakeRotfromX HitNormal) "KeepWorldPosition" 1e+01))

(fn GetRandomImpactMaterial
  (switch int (Math|Random|RandomIntegerinRange 0 1)
    (:Default
      (return "/Game/Asset/Materials/MAT_Impact1.MAT_Impact1"))
    (:0
      (return "/Game/Asset/Materials/MAT_Impact1.MAT_Impact1"))
    (:1
      (return "/Game/Asset/Materials/MAT_Impact2.MAT_Impact2"))))

(fn GetRandomRotation
  (bind _precision (Variables|Default|GetPrecision))
  (bind _returnvalue (- 1e+02 _precision))
  (bind _returnvalue_2 (/ _returnvalue 1e+02))
  (if (< 3e+01 (* (- (Utilities|Time|GetTimeSeconds) (Variables|Default|GetLastShotTime)) 1e+02))
    (Variables|Default|SetShotStreak 1.0)
    (else
      (Math|Float|IncrementFloat (Variables|Default|GetShotStreak)
        (:%20%20
          _))))
  (return (Math|Rotator|MakeRotator 0.0 (* (Math|Random|RandomFloatinRange (* -0.5 (Variables|Default|GetShotStreak)) (* 0.5 (Variables|Default|GetShotStreak))) _returnvalue_2) (* (Math|Random|RandomFloatinRange (* -0.5 (Variables|Default|GetShotStreak)) (* 0.5 (Variables|Default|GetShotStreak))) _returnvalue_2))))